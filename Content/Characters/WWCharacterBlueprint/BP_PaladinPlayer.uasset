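; Paladin player Blueprint that holds what appears to be a debug test of a hit reaction animation.
; Pressing B plays the hit reaction montage directly on the mesh through PlayAnimation, without looping.
; Tick polls that montage's position on the anim instance and, past a threshold, blends it out, returns the mesh to Animation Blueprint mode and prints a debug message.
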(event EventBeginPlay)

(event Collision|EventActorBeginOverlap
  (params (OtherActor :type Actor%20Object%20Reference)))

(event EventTick
  (params (DeltaSeconds :type Float%20%28single-precision%29))
  (bind _mesh (Variables|Character|GetMesh))
  (bind _returnvalue (Components|SkeletalMesh|GetAnimInstance _mesh))
  (if (> (Animation|Montage|MontageGetPosition _returnvalue "/Game/Animations/PaladinPack/PaladinMontages/AM_HitReaction.AM_HitReaction") 0.9)
    (Animation|Montage|MontageStop _returnvalue 1.0 "/Game/Animations/PaladinPack/PaladinMontages/AM_HitReaction.AM_HitReaction")
    (Components|Animation|SetAnimationMode _mesh "AnimationBlueprint")
    (Development|PrintText "Hello")))

(event Input|KeyboardEvents|B
  (params (Key :type Key%20Structure :default "None"))
  (:Pressed
    (Components|Animation|PlayAnimation (Variables|Character|GetMesh) "/Game/Animations/PaladinPack/PaladinMontages/AM_HitReaction.AM_HitReaction" false)))

(fn ConstructionScript)