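; Player character Blueprint that plays the demo's opening Level Sequence and carries some test inputs.
; A one-shot Tick check starts LC_DemoStart, hiding the character, weapon and in-game widget and blocking AI start through WWGameInstance.
; Enter resumes a paused sequence; helper functions wrap playback, visibility and AI gating, with no restore call in this graph.
; Debug inputs make BP_WizardCharacter play its attack montage or move to the player.
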(event EventBeginPlay)

(event Collision|EventActorBeginOverlap
  (params (OtherActor :type Actor%20Object%20Reference)))

(event EventTick
  (params (DeltaSeconds :type Float%20%28single-precision%29))
  (if (Variables|Default|GetWillPlayDemoStartLC)
    (if (not (Variables|Default|GetIsLC_DemoStartPlayed))
      (Variables|Default|SetIsLC_DemoStartPlayed true)
      (bind _returnvalue (Sequencer|Player|CreateLevelSequencePlayer "/Game/Cine/LC_DemoStart.LC_DemoStart"))
      (bind _output_get (Variables|Default|SetCurrentLevelSequencePlayer _returnvalue))
      (Sequencer|Player|Play _output_get :!class /Script/MovieScene.MovieSceneSequencePlayer)
      (CallFunction|HideMyselfinGame true)
      (CallFunction|AlloworNotAIStart false)
      (CallFunction|HideinGameWidget true))))

(event Input|ActionEvents|InputActionTest
  (params (Key :type Key%20Structure :default "None"))
  (:Pressed
    (Development|PrintText "Pressed"))
  (:Released
    (bind _returnvalue (Actor|GetActorOfClass "/Game/Characters/WWCharacterBlueprint/BP_WizardCharacter.BP_WizardCharacter_C"))
    (Animation|Montage|MontagePlay (Components|SkeletalMesh|GetAnimInstance (Variables|/Script/Engine.Character|GetMesh _returnvalue)) "/Game/Animations/WizardRooted/AM_WizardAttack.AM_WizardAttack" 1.0 "MontageLength" 0.0 true)
    (Development|PrintText (Utilities|Text|ToText(String) (Utilities|GetObjectName _returnvalue)))))

(event Input|KeyboardEvents|Up
  (params (Key :type Key%20Structure :default "None"))
  (:Pressed
    (bind _returnvalue (Actor|GetActorOfClass "/Game/Characters/WWCharacterBlueprint/BP_WizardCharacter.BP_WizardCharacter_C"))
    (AI|AIMoveTo (AI|GetAIController _returnvalue) 0 "0, 0, 0" self 5.0 false
      (:OnSuccess
        (Development|PrintText "Hello")))))

(event Input|KeyboardEvents|Enter
  (params (Key :type Key%20Structure :default "None"))
  (bind _currentlevelsequenceplayer (Variables|Default|GetCurrentLevelSequencePlayer))
  (:Pressed
    (if (Class|MovieSceneSequencePlayer|IsPaused _currentlevelsequenceplayer)
      (Sequencer|Player|Play _currentlevelsequenceplayer :!class /Script/MovieScene.MovieSceneSequencePlayer))))

(fn ConstructionScript)

(fn PlayCurrentLevelSequence
  (Sequencer|Player|Play (Variables|Default|GetCurrentLevelSequencePlayer) :!class /Script/MovieScene.MovieSceneSequencePlayer))

(fn HideMyselfinGame
  (params (WillHide :type Boolean))
  (bind _self self)
  (bind _currentweapon (Variables|Default|GetCurrentWeapon _self))
  (Rendering|SetActorHiddenInGame _self WillHide)
  (if (Utilities|IsValid _currentweapon)
    (Rendering|SetActorHiddenInGame _currentweapon WillHide)))

(fn HideinGameWidget
  (params (WillHide :type Boolean))
  (bind _aswwplayer_controller (Utilities|Casting|CastToWWPlayerController (Game|GetPlayerController 0)))
  (Class|WWPlayerController|SetinGameWidgetHide _aswwplayer_controller WillHide))

(fn AlloworNotAIStart
  (params (WillAllowStart :type Boolean))
  (bind _aswwgame_instance (Utilities|Casting|CastToWWGameInstance (Game|GetGameInstance)))
  (Class|WWGameInstance|SetAllowStart _aswwgame_instance WillAllowStart))