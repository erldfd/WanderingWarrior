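; Trigger box that plays cutscene level sequences when BP_PlayerCharacter2 overlaps it.
; The first overlap plays the main sequence and, if a Door is set, calls it to open or close and hides the listed static meshes.
; Later overlaps play the return-to-wizard sequence once the player's flag allows it, then clear that flag.
; Both paths hand the sequence player to the character, hide the character and HUD, and disallow AI start.
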(event EventBeginPlay)

(event Collision|EventActorBeginOverlap
  (params (OtherActor :type Actor%20Object%20Reference))
  (bind _door (Variables|Default|GetDoor))
  (if (Variables|Default|GetIsPlayedFisrtLC)
    (if (Utilities|IsValid (Variables|Default|GetReturnToWizardLC))
      (bind _asbp_player_character_2 (Utilities|Casting|CastToBP_PlayerCharacter2 OtherActor))
      (if (Variables|/Game/Characters/WWCharacterBlueprint/BP_PlayerCharacter2.BP_PlayerCharacter2_C|GetWillPlayReturnToWizardLC _asbp_player_character_2)
        (bind _returnvalue (Sequencer|Player|CreateLevelSequencePlayer (Variables|Default|GetReturnToWizardLC)))
        (Sequencer|Player|Play _returnvalue :!class /Script/MovieScene.MovieSceneSequencePlayer)
        (Variables|/Game/Characters/WWCharacterBlueprint/BP_PlayerCharacter2.BP_PlayerCharacter2_C|SetCurrentLevelSequencePlayer _asbp_player_character_2 _returnvalue)
        (Default|HideinGameWidget _asbp_player_character_2 true)
        (Default|HideMyselfinGame _asbp_player_character_2 true)
        (Default|AlloworNotAIStart _asbp_player_character_2 false)
        (Variables|/Game/Characters/WWCharacterBlueprint/BP_PlayerCharacter2.BP_PlayerCharacter2_C|SetWillPlayReturnToWizardLC _asbp_player_character_2 false)))
    (else
      (bind _asbp_player_character_2_2 (Utilities|Casting|CastToBP_PlayerCharacter2 OtherActor)
        (:then
          (bind _returnvalue_2 (Sequencer|Player|CreateLevelSequencePlayer (Variables|Default|GetLevelSequence)))
          (if (Utilities|IsValid _door)
            (Default|OpenorCloseDoor _door true)
            (for _array_element (Variables|Default|GetStaticMeshActors)
              (Rendering|SetActorHiddenInGame _array_element true)
              (Development|PrintText "Hidden")))
          (Sequencer|Player|Play _returnvalue_2 :!class /Script/MovieScene.MovieSceneSequencePlayer)
          (Variables|/Game/Characters/WWCharacterBlueprint/BP_PlayerCharacter2.BP_PlayerCharacter2_C|SetCurrentLevelSequencePlayer _asbp_player_character_2_2 _returnvalue_2)
          (Default|HideMyselfinGame _asbp_player_character_2_2 true)
          (Default|HideinGameWidget _asbp_player_character_2_2 true)
          (Default|AlloworNotAIStart _asbp_player_character_2_2 false)
          (Variables|Default|SetIsPlayedFisrtLC true))
        (:CastFailed
          (Development|PrintText "CastFailed"))))))

(event EventTick
  (params (DeltaSeconds :type Float%20%28single-precision%29)))

(fn ConstructionScript)