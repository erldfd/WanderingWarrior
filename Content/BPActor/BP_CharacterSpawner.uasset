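; BP_CharacterSpawner is an actor that spawns a set number of characters at its own transform, one per timed interval.
; While activated, Tick accumulates delta time, spawns SpawningCharacter when SpawnTime is reached, and counts spawns against Times.
; Spawned BP_EnemyNormal enemies get rush AI enabled on their EnemyAIController.
; That branch also clears WillSpawnCharacter at the limit, after which the counter resets.
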(event EventBeginPlay)

(event Collision|EventActorBeginOverlap
  (params (OtherActor :type Actor%20Object%20Reference)))

(event EventTick
  (params (DeltaSeconds :type Float%20%28single-precision%29))
  (if (Variables|Default|GetWillActivate)
    (if (and (Variables|Default|GetWillSpawnCharacter) (> (Variables|Default|GetTimes) (Variables|Default|GetCurrentTimes)))
      (if (>= (Variables|Default|GetCollapsedTime) (Variables|Default|GetSpawnTime))
        (Variables|Default|SetCollapsedTime 0.0)
        (bind _returnvalue (Game|SpawnActorfromClass (Variables|Default|GetSpawningCharacter) (Transformation|GetActorTransform self) "Undefined" 0 0))
        (Variables|Default|SetCurrentTimes (+ (Variables|Default|GetCurrentTimes) 1))
        (bind _asbp_enemy_normal (Utilities|Casting|CastToBP_EnemyNormal _returnvalue))
        (bind _asenemy_aicontroller (Utilities|Casting|CastToEnemyAIController (AI|GetAIController _asbp_enemy_normal)))
        (Variables|/Script/WanderingWarrior.EnemyAIController|SetbWillUseRushAI _asenemy_aicontroller true)
        (Variables|Default|SetWillSpawnCharacter (> (Variables|Default|GetTimes) (Variables|Default|GetCurrentTimes)))
        (else
          (Variables|Default|SetCollapsedTime (+ DeltaSeconds (Variables|Default|GetCollapsedTime)))))
      (else
        (Variables|Default|SetCurrentTimes 0)))))

(fn ConstructionScript)