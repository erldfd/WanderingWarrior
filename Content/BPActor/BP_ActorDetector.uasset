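; Detector actor that plays a cutscene once no enemies of a given class remain in the area around it.
; Every Tick, a box overlap searches for the boss or normal enemies, as WillPlayEndOfBossBattle selects.
; When none are found, it plays the matching level sequence once, guarded by a flag.
; It also hides the player and in-game widget, disallows AI start, and hands the sequence player to the player character.
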(event EventBeginPlay)

(event Collision|EventActorBeginOverlap
  (params (OtherActor :type Actor%20Object%20Reference)))

(event EventTick
  (params (DeltaSeconds :type Float%20%28single-precision%29))
  (if (Variables|Default|GetWillPlayEndOfBossBattle)
    (bind _returnvalue (Collision|BoxOverlapActors (Transformation|GetActorLocation) "3000.000000,3000.000000,3000.000000" (Variables|Default|GetObject%20Types) "/Game/Characters/WWCharacterBlueprint/BP_TestBossCharacter.BP_TestBossCharacter_C" :!class /Script/Engine.KismetSystemLibrary))
    (bind _output_get (Variables|Default|SetExistActors _returnvalue))
    (if (not (Variables|Default|GetIsPlayedEndOfBossBattle))
      (if (not _output_get)
        (Variables|Default|SetIsPlayedEndOfBossBattle true)
        (bind _returnvalue_2 (Sequencer|Player|CreateLevelSequencePlayer (Variables|Default|GetLC_EndOfBossBattle)))
        (Sequencer|Player|Play _returnvalue_2 :!class /Script/MovieScene.MovieSceneSequencePlayer)
        (bind _returnvalue_3 (Actor|GetActorOfClass "/Game/Characters/WWCharacterBlueprint/BP_PlayerCharacter2.BP_PlayerCharacter2_C"))
        (Default|HideinGameWidget _returnvalue_3 true)
        (Default|HideMyselfinGame _returnvalue_3 true)
        (Default|AlloworNotAIStart _returnvalue_3 false)
        (Variables|/Game/Characters/WWCharacterBlueprint/BP_PlayerCharacter2.BP_PlayerCharacter2_C|SetCurrentLevelSequencePlayer _returnvalue_3 _returnvalue_2)))
    (else
      (bind _returnvalue_4 (Collision|BoxOverlapActors (Transformation|GetActorLocation) "3000.000000,3000.000000,3000.000000" (Variables|Default|GetObject%20Types) "/Game/Characters/WWCharacterBlueprint/BP_EnemyNormal.BP_EnemyNormal_C" :!class /Script/Engine.KismetSystemLibrary))
      (bind _output_get_2 (Variables|Default|SetExistActors _returnvalue_4))
      (if (not (Variables|Default|GetIsPlayedLC))
        (if (not _output_get_2)
          (Variables|Default|SetIsPlayedLC true)
          (bind _returnvalue_5 (Sequencer|Player|CreateLevelSequencePlayer (Variables|Default|GetLC)))
          (Sequencer|Player|Play _returnvalue_5 :!class /Script/MovieScene.MovieSceneSequencePlayer)
          (bind _returnvalue_6 (Actor|GetActorOfClass "/Game/Characters/WWCharacterBlueprint/BP_PlayerCharacter2.BP_PlayerCharacter2_C"))
          (Default|HideinGameWidget _returnvalue_6 true)
          (Default|HideMyselfinGame _returnvalue_6 true)
          (Default|AlloworNotAIStart _returnvalue_6 false)
          (Variables|/Game/Characters/WWCharacterBlueprint/BP_PlayerCharacter2.BP_PlayerCharacter2_C|SetCurrentLevelSequencePlayer _returnvalue_6 _returnvalue_5))))))

(fn ConstructionScript)